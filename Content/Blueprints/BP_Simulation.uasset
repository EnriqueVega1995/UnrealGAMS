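; Simulation manager that spawns robot agents (quadcopter, tank, car, fixed-wing, satellite) on request from OSC messages.
; Received messages are queued and Tick handles one per frame, mapping the address to a Blueprint class path built from the agent name.
; A JSON blob supplies transform, port and ID; CheckIpAndPort blocks and reserves against duplicate ports or IDs.
; The spawned SimPawn receives its port and ID.
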(event `self.ReceiveBeginPlay`
  (add `OscReceiverComponent.OnOscReceived` (`self.OscReceiver`) (delegate `onReceivedOSC`)))

(event `onReceivedOSC`
  (params (Address :type "Name (by ref)") (Data :type "Array of OscDataElemStruct Structure (by ref)") (SenderIp :type String))
  (`KismetArrayLibrary.Array_Add` (`self.SpawnQueue`) (make `/Game/Blueprints/ST_SpawnEvent` Address Data)))

(event `self.ReceiveTick`
  (params (DeltaSeconds :type "Float (single-precision)"))
  (bind _spawnqueue (`self.SpawnQueue`))
  (bind (_output_address _output_data) (break `/Game/Blueprints/ST_SpawnEvent` (`|GetArrayItem` _spawnqueue)))
  (if (> (`KismetArrayLibrary.Array_Length` _spawnqueue) 0)
    (`self.Spawn` _output_address _output_data)
    (`KismetArrayLibrary.Array_Remove` _spawnqueue)))

(fn `Spawn`
  (params (Address :type Name) (Data :type "Array of OscDataElemStruct Structure"))
  (bind _returnvalue (`BlueprintJsonLibrary.Conv_StringToJsonObject` (`LowEntryExtendedStandardLibrary.BytesToStringUtf8` (`.Value` (`OscFunctionLibrary.PopBlob` Data)))))
  (bind _returnvalue_2 (`BlueprintJsonLibrary.Conv_JsonValueToObject` (`BlueprintJsonLibrary.Conv_JsonObjectToJsonValue` _returnvalue "rotation")))
  (bind _returnvalue_3 (`BlueprintJsonLibrary.Conv_JsonValueToObject` (`BlueprintJsonLibrary.Conv_JsonObjectToJsonValue` _returnvalue "location")))
  (bind _returnvalue_4 (`BlueprintJsonLibrary.Conv_JsonValueToString` (`BlueprintJsonLibrary.Conv_JsonObjectToJsonValue` _returnvalue "port")))
  (bind _returnvalue_5 (`BlueprintJsonLibrary.Conv_JsonValueToString` (`BlueprintJsonLibrary.Conv_JsonObjectToJsonValue` _returnvalue "id")))
  (bind _returnvalue_6 (`KismetStringLibrary.Conv_StringToName` _returnvalue_4))
  (bind _returnvalue_7 (`KismetStringLibrary.Conv_StringToName` _returnvalue_5))
  (switch `name` Address
    (:`/spawn/quadcopter`
      (set `self.AgentName` "Quadcopter"))
    (:`/spawn/tank`
      (set `self.AgentName` "Tank"))
    (:`/spawn/car`
      (set `self.AgentName` "Car"))
    (:`/spawn/fixedwing`
      (set `self.AgentName` "FixedWing"))
    (:`/spawn/satellite`
      (set `self.AgentName` "Satellite")))
  (if (or (`BlueprintSetLibrary.Set_Contains` (`self.ReservedPorts`) _returnvalue_6) (`BlueprintSetLibrary.Set_Contains` (`self.ReservedIds`) _returnvalue_7))
    (`KismetSystemLibrary.PrintString` (`KismetTextLibrary.Conv_TextToString` (`|FormatText` "Duplicate PORT or ID: ID={id}, PORT={port}" (`KismetTextLibrary.Conv_StringToText` _returnvalue_4) (`KismetTextLibrary.Conv_StringToText` _returnvalue_5))))
    (else
      (`BlueprintSetLibrary.Set_Add` (`self.ReservedPorts`) _returnvalue_6)
      (`BlueprintSetLibrary.Set_Add` (`self.ReservedIds`) _returnvalue_7)
      (bind (_class_ _success) (`LowEntryExtendedStandardLibrary.GetClassWithName` (`KismetTextLibrary.Conv_TextToString` (`|FormatText` "/Game/Robots/{agent}/Blueprints/BP_{agent}.BP_{agent}_C" (`self.AgentName`)))))
      (if _success
        (bind _asactor (castclass `Actor` _class_))
        (bind _returnvalue_8 (`|SpawnActorFromClass` _asactor (`KismetMathLibrary.MakeTransform` (`KismetMathLibrary.MakeVector` (`BlueprintJsonLibrary.Conv_JsonValueToFloat` (`BlueprintJsonLibrary.Conv_JsonObjectToJsonValue` _returnvalue_3 "x")) (`BlueprintJsonLibrary.Conv_JsonValueToFloat` (`BlueprintJsonLibrary.Conv_JsonObjectToJsonValue` _returnvalue_3 "y")) (`BlueprintJsonLibrary.Conv_JsonValueToFloat` (`BlueprintJsonLibrary.Conv_JsonObjectToJsonValue` _returnvalue_3 "z"))) (`KismetMathLibrary.MakeRotator` (`BlueprintJsonLibrary.Conv_JsonValueToFloat` (`BlueprintJsonLibrary.Conv_JsonObjectToJsonValue` _returnvalue_2 "x")) (`BlueprintJsonLibrary.Conv_JsonValueToFloat` (`BlueprintJsonLibrary.Conv_JsonObjectToJsonValue` _returnvalue_2 "y")) (`BlueprintJsonLibrary.Conv_JsonValueToFloat` (`BlueprintJsonLibrary.Conv_JsonObjectToJsonValue` _returnvalue_2 "z")))) "Undefined" "OverrideRootScale" null null))
        (bind _assim_pawn (cast `/Game/Common/Blueprints/SimPawn` _returnvalue_8))
        (set `/Game/Common/Blueprints/SimPawn.AgentPort` (`KismetStringLibrary.Conv_StringToName` (`BlueprintJsonLibrary.Conv_JsonValueToString` (`BlueprintJsonLibrary.Conv_JsonObjectToJsonValue` _returnvalue "port"))) _assim_pawn)
        (set `/Game/Common/Blueprints/SimPawn.AgentId` (`KismetStringLibrary.Conv_StringToName` (`BlueprintJsonLibrary.Conv_JsonValueToString` (`BlueprintJsonLibrary.Conv_JsonObjectToJsonValue` _returnvalue "id"))) _assim_pawn)
        (else
          (`KismetSystemLibrary.PrintString` "Failure! Class couldn't be found."))))))

(fn `UserConstructionScript`)