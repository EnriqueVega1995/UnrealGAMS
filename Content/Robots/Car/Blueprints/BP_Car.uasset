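; Drivable car pawn with orbit cameras, switchable lights and OSC remote control.
; Tick and input axes feed throttle and steering, while mesh torques fake pitch, roll and gear-shift inertia.
; OSC messages set acceleration and steering, and OscTick sends position and rotation back.
; Engine audio, camera switching, steering animation and character entry are unwired, and the exit function is never called here.
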(event `self.ReceivePossessed`
  (params (NewController :type "Controller Object Reference"))
  ;[1 1 1] Vehicle Sounds
  ;;[1 1 1] Activate the Sound
)

(event `self.ReceiveTick`
  (params (DeltaSeconds :type "Float (single-precision)"))
  (bind _moveforward (`self.MoveForward`))
  ;[1 1 1] Vehicle Sounds
  ;;[1 1 1] Setting the RPM / Modulating the Engine Sound at various Rpm values
  (`|ExecutionSequence`
    (:`then_0`
      ;[1 1 1] Basic Car Controls
      (`|ExecutionSequence` :!label _label
        (:`then_0`
          (`WheeledVehicleMovementComponent.SetThrottleInput` (`self.VehicleMovement`) _moveforward)
          ;[1 1 1] Lights / front and rear lights by pressing L key or brakelights of the car
          (`self.LightsBraked` _moveforward (stale `Key|L` _output_get)))
        (:`then_1`
          ;[1 1 1] Clutch Effect / shift the gear with inertial behaviour
          (`self.ClutchEffect` _moveforward _moveforward _moveforward))
        (:`then_2`
          ;[1 1 1] Car Pitch / Car reaction while accelerating and braking
          (`self.CarPitch` _moveforward _moveforward :!label _label_2))
        (:`then_3`
          (goto _label_2 :!via `execute2`))
        (:`then_4`
          ;[1 1 1] Car Roll / It calculates the behaviour of the turning right and left
          (`self.CarRoll`))
        (:`then_5`)
        (:`then_6`)))
    (:`then_1`
      (`WheeledVehicleMovementComponent.SetSteeringInput` (`self.VehicleMovement`) (`self.Direction`) :!label _label_3))))

(event `InputAxisKey|MouseX`
  (params (AxisValue :type "Float (single-precision)"))
  ;[1 1 1] Mouse Cam / It turns the camera around the car with Mouse
  (`self.CamOrbit` AxisValue (stale `InputAxisKey|MouseY` AxisValue) :!label _label_4))

(event `InputAxisKey|MouseY`
  (params (AxisValue :type "Float (single-precision)"))
  ;[1 1 1] Mouse Cam / It turns the camera around the car with Mouse
  (goto _label_4 :!via `execute2`))

(event `Key|One`
  (params (Key :type "Key Structure"))
  ;[1 1 1] Cam1 / Outer Camera of the Car
)

(event `Key|R`
  (params (Key :type "Key Structure"))
  ;[1 1 1] Car Reset
  (:`Pressed`
    (`SceneComponent.K2_SetRelativeRotation` :`self` (`self.Mesh`) :`bTeleport` true)))

(event `Key|MouseScrollDown`
  (params (Key :type "Key Structure"))
  ;[1 1 1] Mouse Cam / It turns the camera around the car with Mouse
  (:`Pressed`
    (`self.CamZoom` :!label _label_5)))

(event `Key|Two`
  (params (Key :type "Key Structure"))
  ;[1 1 1] Cam2 / Interior Camera of the Car
)

(event `Key|MouseScrollUp`
  (params (Key :type "Key Structure"))
  ;[1 1 1] Mouse Cam / It turns the camera around the car with Mouse
  (:`Pressed`
    (goto _label_5 :!via `execute2`)))

(event `InputAxisKey|Gamepad_RightX`
  (params (AxisValue :type "Float (single-precision)"))
  ;[1 1 1] Camera Orbit
  (`self.CamOrbit` AxisValue (stale `InputAxisKey|Gamepad_RightY` AxisValue) :!label _label_6))

(event `self.ReceiveBeginPlay`
  ;[1 1 1] OSC
  ;;[1 1 1] OSC SetUp
  (add `OscReceiverComponent.OnOscReceived` (`self.OscReceiver`) (delegate `OnReceiveOSC`)))

(event `InputAxisKey|Gamepad_RightY`
  (params (AxisValue :type "Float (single-precision)"))
  ;[1 1 1] Camera Orbit
  (goto _label_6 :!via `execute2`))

(event `self.ReceiveEndPlay`
  (params (EndPlayReason :type "EEndPlayReason Enum" :default "Destroyed"))
  ;[1 1 1] OSC
  ;;[1 1 1] OSC SetUp
  (remove `OscReceiverComponent.OnOscReceived` (`self.OscReceiver`) (delegate `OnReceiveOSC`)))

(event `OnReceiveOSC`
  (params (Address :type "Name (by ref)") (Data :type "Array of OscDataElemStruct Structure (by ref)") (SenderIp :type String))
  ;[1 1 1] OSC
  ;;[1 1 1] OSC SetUp
  (`/OSC/Blueprints/OscSender.SetupOSCSender` (`self.OscSender`) true Address SenderIp (`self.AgentPort`))
  (if (`self.OSCTicking`)
    (switch `name` Address
      (:`/acceleration`
        (set `self.MoveForward` (`.Value` (`OscFunctionLibrary.PopFloat` Data)) :!label _label_7))
      (:`/move`
        (set `self.Direction` (`.Value` (`OscFunctionLibrary.PopFloat` Data)))))
    (else
      (goto _label_7))))

(event `Key|L`
  (params (Key :type "Key Structure"))
  ;[1 1 1] Lights / front and rear lights by pressing L key or brakelights of the car
  (:`Pressed`
    (bind _output_get (`self.Lights`))))

(event `/OSC/Blueprints/OscSenderInterface.OscTick`
  (bind _oscsender (`self.OscSender`))
  (bind _oscsender_2 (`self.OscSender`))
  ;[1 1 1] OSC
  ;;[1 1 1] Send position and rotation
  (bind _output (`/OSC/Blueprints/OscSender.PushVector` _oscsender_2 (`self.K2_GetActorLocation`)))
  (`/OSC/Blueprints/OscSender.AddOSCMessage` _oscsender_2 (`self.AgentId`) "pos" _output)
  (bind _output_2 (`/OSC/Blueprints/OscSender.PushEuler` _oscsender (`self.K2_GetActorRotation`)))
  (`/OSC/Blueprints/OscSender.AddOSCMessage` _oscsender (`self.AgentId`) "rot" _output_2)
  (`/OSC/Blueprints/OscSender.SendOSCMessages` (`self.OscSender`)))

(event `InputAxis|MoveForward`
  (params (AxisValue :type "Float (single-precision)"))
  ;[1 1 1] Basic Car Controls
  (goto _label))

(event `InputAxis|MoveRight`
  (params (AxisValue :type "Float (single-precision)"))
  ;[1 1 1] Basic Car Controls
  (goto _label_3))

(event `self.Trigger.OnComponentBeginOverlap`
  (params (OverlappedComponent :type "PrimitiveComponent Object Reference") (OtherActor :type "Actor Object Reference") (OtherComp :type "PrimitiveComponent Object Reference") (OtherBodyIndex :type Integer) (bFromSweep :type Boolean) (SweepResult :type "HitResult Structure (by ref)"))
  ;[1 1 1] Trigger for the Vehicle interaction. It checks, if the character is in the Collider or not
)

(event `self.Trigger.OnComponentEndOverlap`
  (params (OverlappedComponent :type "PrimitiveComponent Object Reference") (OtherActor :type "Actor Object Reference") (OtherComp :type "PrimitiveComponent Object Reference") (OtherBodyIndex :type Integer))
  ;[1 1 1] Trigger for the Vehicle interaction. It checks, if the character is in the Collider or not
)

(fn `UserConstructionScript`)