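; BP_TankMissile is a tank missile projectile that handles the exit from its bullet camera and its own cleanup.
; Shortly after spawning it records whether its owner is the player's pawn, then starts a lifetime timeout.
; Timeout, impact, or Escape on a player missile triggers a one-shot return of the player's view to the owner, then delayed destruction.
; Impact also spawns an emitter once at the missile's location.
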(event `self.ReceiveBeginPlay`
  ;[1 1 1] STart Bullet Trace
  (`KismetSystemLibrary.Delay` 1.0)
  (set `self.CharacterBullet` (== (`Controller.K2_GetPawn` (`GameplayStatics.GetPlayerController` 0)) (`self.GetOwner`)))
  ;[1 1 1] Time Out for bullet view
  (`KismetSystemLibrary.Delay` (`self.BulletMaxLifetime`))
  (`self.EventBackToOwner`))

(event `EventBackToOwner`
  (bind _returnvalue (`GameplayStatics.GetPlayerController` 0))
  (bind _returnvalue_2 (`self.GetOwner`))
  ;[1 1 1] Back to original pawn
  (`/Engine/EditorBlueprintResources/StandardMacros.DoOnce` false
    (:`Completed`
      (`/Engine/EditorBlueprintResources/StandardMacros.IsValid` _returnvalue_2
        (:`Is Valid`
          (if (== (`Controller.K2_GetPawn` _returnvalue) _returnvalue_2)
            (`PlayerController.SetViewTargetWithBlend` _returnvalue _returnvalue_2 0.0 "VTBlend_Linear" 0.0 false))
          (`KismetSystemLibrary.Delay` 0.5)
          (`self.K2_DestroyActor`))))))

(event `self.ReceiveHit`
  (params (MyComp :type "PrimitiveComponent Object Reference") (Other :type "Actor Object Reference") (OtherComp :type "PrimitiveComponent Object Reference") (bSelfMoved :type Boolean) (HitLocation :type "Vector Structure") (HitNormal :type "Vector Structure") (NormalImpulse :type "Vector Structure") (Hit :type "HitResult Structure (by ref)"))
  ;[1 1 1] Event Hit
  (set `self.Hit` true)
  (`/Engine/EditorBlueprintResources/StandardMacros.DoOnce` false
    (:`Completed`
      (`self.EventBackToOwner`)
      (`GameplayStatics.SpawnEmitterAtLocation` null (`self.K2_GetActorLocation`)))))

(event `self.ReceiveTick`
  (params (DeltaSeconds :type "Float (single-precision)"))
  ;[1 1 1] Exit Bullet Camera
  (if (`self.CharacterBullet`)
    (if (`PlayerController.IsInputKeyDown` (`GameplayStatics.GetPlayerController` 0) "Escape")
      (`self.EventBackToOwner`))))

(fn `UserConstructionScript`)