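; BP_Satellite is a robot satellite steered remotely over OSC.
; Received messages on agent-prefixed addresses set horizontal and vertical control input and point the sender at the sending IP.
; Each tick rotates that input by camera yaw and adds it, scaled by speed and delta time, to the physics box's velocity.
; OscTick sends the box's position and rotation back over OSC.
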(event `self.ReceiveTick`
  (params (DeltaSeconds :type "Float (single-precision)"))
  ;[1 1 1] Satellite controls
  (`PrimitiveComponent.SetPhysicsLinearVelocity` (`self.Box`) (+ (`self.GetVelocity`) (* (* (`KismetMathLibrary.GreaterGreater_VectorRotator` (`KismetMathLibrary.MakeVector` (`self.ControlVelocityY`) (`self.ControlVelocityX`) (`self.ControlVelocityZ`)) (`KismetMathLibrary.MakeRotator` 0.0 0.0 (.yaw (`SceneComponent.K2_GetComponentRotation` (`self.Camera`))))) (`self.MovementSpeed`)) DeltaSeconds)) false "None"))

(event `self.ReceiveEndPlay`
  (params (EndPlayReason :type "EEndPlayReason Enum" :default "Destroyed"))
  ;[0.3341 0.371 0.4688] OSC
  ;;[1 1 1] Setup
  (remove `OscReceiverComponent.OnOscReceived` (`self.OscReceiver`) (delegate `OnReceiveOSC`)))

(event `self.ReceiveBeginPlay`
  ;[0.3341 0.371 0.4688] OSC
  ;;[1 1 1] Setup
  (add `OscReceiverComponent.OnOscReceived` (`self.OscReceiver`) (delegate `OnReceiveOSC`)))

(event `OnReceiveOSC`
  (params (Address :type "Name (by ref)") (Data :type "Array of OscDataElemStruct Structure (by ref)") (SenderIp :type String))
  (bind _returnvalue (`KismetArrayLibrary.Array_Find` (`self.Addresses`) Address))
  ;[0.3341 0.371 0.4688] OSC
  ;;[1 1 1] Setup
  (`/OSC/Blueprints/OscReceiver.PrefixAddresses` (`self.OscReceiver`) (`self.AgentId`) (`self.Addresses`))
  (`/OSC/Blueprints/OscSender.SetupOSCSender` (`self.OscSender`) true Address SenderIp (`self.AgentPort`))
  ;;[1 1 1] Handling received OSC Messages
  (if (> _returnvalue -1)
    (switch `int` _returnvalue
      (:`0`
        (bind _vector (`/OSC/Blueprints/OscReceiver.popVector2D` (`self.OscReceiver`) Data))
        (set `self.ControlVelocityX` (`KismetMathLibrary.BreakVector2D` _vector))
        (set `self.ControlVelocityY` (`.Y` (`KismetMathLibrary.BreakVector2D` _vector))))
      (:`1`
        (set `self.ControlVelocityZ` (`.Value` (`OscFunctionLibrary.PopFloat` Data)))))))

(event `/OSC/Blueprints/OscSenderInterface.OscTick`
  (bind _oscsender (`self.OscSender`))
  (bind _oscsender_2 (`self.OscSender`))
  ;[0.3341 0.371 0.4688] OSC
  ;;[1 1 1] Sending back position and rotation
  (bind _output (`/OSC/Blueprints/OscSender.PushVector` _oscsender (`SceneComponent.K2_GetComponentLocation` (`self.Box`))))
  (`/OSC/Blueprints/OscSender.AddOSCMessage` _oscsender (`self.AgentId`) "pos" _output)
  (bind _output_2 (`/OSC/Blueprints/OscSender.PushEuler` _oscsender_2 (`SceneComponent.K2_GetComponentRotation` (`self.Box`))))
  (`/OSC/Blueprints/OscSender.AddOSCMessage` _oscsender_2 (`self.AgentId`) "rot" _output_2)
  (`/OSC/Blueprints/OscSender.SendOSCMessages` (`self.OscSender`)))

(fn `UserConstructionScript`)