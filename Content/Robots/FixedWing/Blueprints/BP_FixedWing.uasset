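; Fixed-wing aircraft robot that an external agent controls remotely over OSC.
; Incoming messages point the OSC sender at the caller's IP, then set EasyFM flight-model pitch, roll and yaw inputs by address.
; Acceleration messages instead apply a scaled throttle force along world X to the skeletal mesh, once per message received.
; OscTick sends the actor's position and rotation back, tagged with its agent ID.
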(event Custom|OnReceiveOSC
  (params (Address :type Name%20%28by%20ref%29) (Data :type Array%20of%20Osc%20Data%20Elem%20Struct%20Structures) (SenderIp :type String))
  (bind _easyfm (Variables|Default|GeteasyFM))
  ;[1 1 1] OSC Setup
  (Default|SetupOSCSender (Variables|Default|GetOscSender) true Address SenderIp (Variables|OSC|GetAgent%20Port))
  (Development|PrintString (|OSCMessageDetails Address SenderIp))
  (switch name Address
    (:/agent/pitch/y
      (Variables|/Script/EasyFM.easyFM|SetPitchInput _easyfm (.Value (Class|OscFunctionLibrary|PopFloat Data))))
    (:/agent/roll/x
      (Variables|/Script/EasyFM.easyFM|SetRollInput _easyfm (.Value (Class|OscFunctionLibrary|PopFloat Data))))
    (:/agent/yaw/x
      (Variables|/Script/EasyFM.easyFM|SetYawInput _easyfm (.Value (Class|OscFunctionLibrary|PopFloat Data))))
    (:/agent/acceleration/x
      (bind _output_get (Variables|Default|SetThrottle (.Value (Class|OscFunctionLibrary|PopFloat Data))))
      (Physics|AddForce (Variables|Default|GetSkeletalMesh) (Math|Vector|MakeVector (|(x*y) _output_get 6e+06) 0.0 0.0) "None" false))))

(event EventBeginPlay
  ;[1 1 1] OSC Setup
  (EventDispatchers|AssignOnOscReceived (Variables|Default|GetOscReceiver) (delegate Custom|OnReceiveOSC)))

(event EventEndPlay
  (params (EndPlayReason :type EEndPlayReason%20Enum :default "Destroyed"))
  ;[1 1 1] OSC Setup
  (EventDispatchers|UnbindallEventsfromOnOscReceived (Variables|Default|GetOscReceiver)))

(event EventOscTick
  (bind _oscsender (Variables|Default|GetOscSender))
  (bind _oscsender_2 (Variables|Default|GetOscSender))
  (bind _output (Default|PushVector _oscsender (Transformation|GetActorLocation)))
  (Default|AddOSCMessage _oscsender (Variables|OSC|GetAgent%20Id) "pos" _output)
  (bind _output_2 (Default|PushEuler _oscsender_2 (Transformation|GetActorRotation)))
  (Default|AddOSCMessage _oscsender_2 (Variables|OSC|GetAgent%20Id) "rot" _output_2)
  (Default|SendOSCMessages (Variables|Default|GetOscSender)))

(fn ConstructionScript)